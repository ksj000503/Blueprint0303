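; BlueFunLib is a Blueprint function library with two functions that sum a range of numbers between two inputs.
; MyAdd uses a for loop to accumulate every index from Num1 through Num2, inclusive.
; MyAdd2 uses recursion, incrementing Num1 before each self-call and adding it to the returned total until it reaches Num2.
; Unlike the loop version, the recursive sum leaves out the starting Num1.
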(fn MyAdd
  (params (Num1 :type Integer) (Num2 :type Integer))
  (for _index (range Num1 Num2)
    (LocalVariables|SetResult (+ _index (LocalVariables|GetResult))))
  (return (LocalVariables|GetResult)))

(fn MyAdd2
  (params (Num1 :type Integer) (Num2 :type Integer))
  (if (< Num1 Num2)
    (Math|Integer|IncrementInt Num1
      (:%20%20
        (bind _result (CallFunction|MyAdd2 Num1 Num2))
        (bind _output_get (LocalVariables|SetSum (+ _result Num1)))
        (return _output_get)))
    (else
      (return (LocalVariables|GetSum)))))