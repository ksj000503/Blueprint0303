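; Carpet actor that bobs back and forth along its own up axis, like a floating magic carpet.
; Each tick it accumulates running time and feeds it, scaled by MoveSpeed, into a sine wave.
; The result, scaled by MoveDistancs, offsets StartLocation along the Carpet component's up vector, and the actor is moved there without sweeping.
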(event EventTick
  (params (DeltaSeconds :type Float%20%28single-precision%29))
  (bind _output_get (Variables|Default|SetRunning%20Time (+ DeltaSeconds (Variables|Default|GetRunning%20Time))))
  (Transformation|SetActorLocation (+ (Variables|Default|GetStart%20Location) (* (Math|Vector|GetUpVector (Variables|Default|GetCarpet)) (* (Math|Trig|Sin(Radians) (* _output_get (Variables|Default|GetMove%20Speed))) (Variables|Default|GetMove%20Distancs)))) false false))

(fn ConstructionScript)