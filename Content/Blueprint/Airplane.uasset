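; Player-controlled airplane that flies constantly along the actor's forward vector and is steered by input axes.
; Tick sets the actor location from AirplaneSpeed and delta time, without sweep, so the move does no collision check.
; Turn, RightLeft and UpDown apply local pitch, yaw and roll respectively to the Airplane component, all scaled by TuenSpeed and delta time.
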(event EventTick
  (params (DeltaSeconds :type Float%20%28single-precision%29))
  (Transformation|SetActorLocation (+ (Transformation|GetActorLocation) (* (Transformation|GetActorForwardVector) (* (Utilities|Time|GetWorldDeltaSeconds) (Variables|Default|GetAirplaneSpeed)))) false false))

(event Input|AxisEvents|InputAxisRightLeft
  (params (AxisValue :type Float%20%28single-precision%29))
  (if (!= AxisValue 0.0)
    (Transformation|AddLocalRotation (Variables|Default|Getairplane) (Math|Rotator|MakeRotator 0.0 0.0 (* AxisValue (* (Utilities|Time|GetWorldDeltaSeconds) (Variables|Default|GetTuenSpeed)))) false false)))

(event Input|AxisEvents|InputAxisUpDown
  (params (AxisValue :type Float%20%28single-precision%29))
  (if (!= AxisValue 0.0)
    (Transformation|AddLocalRotation (Variables|Default|Getairplane) (Math|Rotator|MakeRotator (* AxisValue (* (Utilities|Time|GetWorldDeltaSeconds) (Variables|Default|GetTuenSpeed))) 0.0 0.0) false false)))

(event Input|AxisEvents|InputAxisTurn
  (params (AxisValue :type Float%20%28single-precision%29))
  (if (!= AxisValue 0.0)
    (Transformation|AddLocalRotation (Variables|Default|Getairplane) (Math|Rotator|MakeRotator 0.0 (* AxisValue (* (Utilities|Time|GetWorldDeltaSeconds) (Variables|Default|GetTuenSpeed))) 0.0) false false)))

(fn ConstructionScript)