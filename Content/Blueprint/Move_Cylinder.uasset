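; Move_Cylinder is an actor Blueprint that slides back and forth in the level, apparently as a moving cylinder prop or obstacle.
; Each tick it accumulates running time and offsets the actor's location along the ModeCylinder component's right vector by a sine of time, scaled by MoveSpeed and MoveDistance.
; The offset adds to the current location every frame without sweeping, so the travel range depends on frame rate.
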(event EventTick
  (params (DeltaSeconds :type Float%20%28single-precision%29))
  (bind _output_get (Variables|Default|SetRunning%20Time (+ DeltaSeconds (Variables|Default|GetRunning%20Time))))
  (Transformation|SetActorLocation (+ (Transformation|GetActorLocation) (* (Math|Vector|GetRightVector (Variables|Default|GetModeCylinder)) (* (Math|Trig|Sin(Radians) (* _output_get (Variables|Default|GetMove%20Speed))) (Variables|Default|GetMove%20Distance)))) false false))

(fn ConstructionScript)